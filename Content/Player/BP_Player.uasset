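; Player Blueprint that gives the player a toggleable inventory screen.
; On BeginPlay it creates a WB_Inventory widget bound to its InventoryComponent with a fixed tile size and keeps the reference.
; The ToggleInventory input adds or removes that same widget from the viewport, switching between Game and UI input with a visible cursor and game-only input with the cursor hidden.
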(event `self.ReceiveBeginPlay`
  (bind _returnvalue (`|CreateWidget` "/Game/Widgets/WB_Inventory.WB_Inventory_C" (`GameplayStatics.GetPlayerController` 0) (`self.InventoryComponent`) 50.0))
  (set `self.InventoryWidget` _returnvalue))

(event `InputAction|ToggleInventory`
  (params (Key :type "Key Structure"))
  (bind _returnvalue (`GameplayStatics.GetPlayerController` 0))
  (bind _returnvalue_2 (`GameplayStatics.GetPlayerController` 0))
  (bind _inventorywidget (`self.InventoryWidget`))
  (:`Pressed`
    (if (`Widget.IsInViewport` (`self.InventoryWidget`))
      (`Widget.RemoveFromParent` _inventorywidget)
      (`WidgetBlueprintLibrary.SetInputMode_GameOnly` _returnvalue_2)
      (set `PlayerController.bShowMouseCursor` false _returnvalue)
      (else
        (`UserWidget.AddToViewport` _inventorywidget 0)
        (`WidgetBlueprintLibrary.SetInputMode_GameAndUIEx` _returnvalue_2 (`self.InventoryWidget`) "DoNotLock" false)
        (set `PlayerController.bShowMouseCursor` true _returnvalue)))))

(fn `UserConstructionScript`)